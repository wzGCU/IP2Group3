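; Trash can obstacle that gets knocked away and adds noise to DrunkGameState when a ThirdPersonCharacter first overlaps it.
; The hit fires once, playing a sound, then launching the mesh after a short delay and switching its collision channel.
; On BeginPlay the authority rolls a random value that tags the can as visibility-based for P1 or P2.
; TrashShow and TrashClearMesh set or clear the can and lid meshes.
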(event `TrashClearMesh`
  (`StaticMeshComponent.SetStaticMesh` (`self.ProperMesh`) null)
  (`StaticMeshComponent.SetStaticMesh` (`self.ProperMeshLid`) null))

(event `TrashShow`
  (`StaticMeshComponent.SetStaticMesh` (`self.ProperMesh`) "/Game/Meshes/Final/ObstaclesNCollectibles/C24_Trashcan.C24_Trashcan")
  (`StaticMeshComponent.SetStaticMesh` (`self.ProperMeshLid`) "/Game/Meshes/Final/ObstaclesNCollectibles/C24_TrashcanLid.C24_TrashcanLid"))

(event `self.ReceiveActorBeginOverlap`
  (params (OtherActor :type "Actor Object Reference"))
  (bind _propermesh (`self.ProperMesh`))
  (if (== (`GameplayStatics.GetObjectClass` OtherActor) "/Game/Blueprints/ThirdPersonCharacter.ThirdPersonCharacter_C")
    (if (not (`self.Hit`))
      (set `self.Hit` true)
      (bind _asdrunk_game_state (cast `/Game/Blueprints/GameMode/DrunkGameState` (`GameplayStatics.GetGameState`)))
      (`/Engine/EditorBlueprintResources/StandardMacros.DoOnce` false
        (:`Completed`
          (`/Game/Blueprints/GameMode/DrunkGameState.AddToNoise` _asdrunk_game_state 0.2)
          (`GameplayStatics.PlaySoundAtLocation` "/Game/Audios/ObstacleHit.ObstacleHit" (`SceneComponent.K2_GetComponentScale` (`self.ProperMesh`)) (struct) 1.0 1.0 0.0 null null null)
          (`KismetSystemLibrary.Delay` 0.2)
          (`PrimitiveComponent.AddForce` _propermesh (0.0 200000.0 99000.0) "None" true)
          (`PrimitiveComponent.SetCollisionObjectType` _propermesh "ECC_GameTraceChannel1"))))))

(event `self.ReceiveBeginPlay`
  (bind _returnvalue (`ActorComponent.GetOwner` (`self.StaticMeshComponent`)))
  (`KismetSystemLibrary.Delay` 0.2)
  (`/Engine/EditorBlueprintResources/ActorMacros.Switch Has Authority`
    (:`Authority`
      (set `self.RandomAssign` (`KismetMathLibrary.RandomFloatInRange` 0.0 100.0)))
    (:`Remote`
      (`KismetSystemLibrary.Delay` 0.2)))
  (if (> (`self.RandomAssign`) 50.0)
    (set `Actor.Tags` (`|MakeArray` "VisibilityBased" "P1Vis" :!type "Name") _returnvalue)
    (else
      (set `Actor.Tags` (`|MakeArray` "VisibilityBased" "P2Vis" :!type "Name") _returnvalue))))

(fn `UserConstructionScript`)