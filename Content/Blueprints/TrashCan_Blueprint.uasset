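; TrashCan_Blueprint is a trash can obstacle that raises the game's noise level when the player bumps into it.
; A TrashShow event assigns the Trash static mesh to ProperMesh.
; Overlap by the ThirdPersonCharacter passes a DoOnce gate, adds to DrunkGameState's noise value, plays a hit sound and destroys the actor.
; The sound's location is fed from the mesh's world scale rather than its position.
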(event `TrashShow`
  (`StaticMeshComponent.SetStaticMesh` (`self.ProperMesh`) "/Game/Meshes/Placeholders/Trash.Trash"))

(event `self.ReceiveActorBeginOverlap`
  (params (OtherActor :type "Actor Object Reference"))
  (if (== (`GameplayStatics.GetObjectClass` OtherActor) "/Game/Blueprints/ThirdPersonCharacter.ThirdPersonCharacter_C")
    (bind _asdrunk_game_state (cast `/Game/Blueprints/GameMode/DrunkGameState` (`GameplayStatics.GetGameState`)))
    (`/Engine/EditorBlueprintResources/StandardMacros.DoOnce` false
      (:`Completed`
        (set `/Game/Blueprints/GameMode/DrunkGameState.NoiseCurrentValue` (+ (`/Game/Blueprints/GameMode/DrunkGameState.NoiseCurrentValue` _asdrunk_game_state) 0.2) _asdrunk_game_state)
        (`GameplayStatics.PlaySoundAtLocation` "/Game/Throwaways/ObstacleHit.ObstacleHit" (`SceneComponent.K2_GetComponentScale` (`self.ProperMesh`)) (struct) 1.0 1.0 0.0 null null null)
        (`self.K2_DestroyActor`)))))

(fn `UserConstructionScript`)