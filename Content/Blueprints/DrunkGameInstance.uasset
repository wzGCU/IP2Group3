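; Game instance for the Drunk game that manages multiplayer sessions, level travel and pausing.
; It hosts a listen-server lobby with a custom session name, joins sessions, and destroys the session on network errors, returning to the main menu.
; Map changes use servertravel console commands, passing through a timed DayNightTravel map before the target level.
; It then starts the DrunkGameMode countdown, retrying the cast until that game mode is available.
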(event `DestroySession`
  (`DestroySessionCallbackProxy.DestroySession` (`GameplayStatics.GetPlayerController` 0)
    (:`OnSuccess`
      (`GameplayStatics.OpenLevelBySoftObjectPtr` "/Game/Maps/MainMenu.MainMenu"))
    (:`OnFailure`
      (`KismetSystemLibrary.PrintString` "Failed to destroy session"))))

(event `HostSession`
  (params (InText :type "Text (by ref)"))
  (`CreateSessionCallbackProxyAdvanced.CreateAdvancedSession` (`|MakeArray` (`AdvancedSessionsLibrary.MakeLiteralSessionPropertyString` "DrunkName" (`KismetTextLibrary.Conv_TextToString` InText))) (`GameplayStatics.GetPlayerController` 0) 4 4
    (:`OnSuccess`
      (`GameplayStatics.OpenLevelBySoftObjectPtr` "/Game/Maps/DrunkLobby.DrunkLobby" true "?listen"))
    (:`OnFailure`
      (`KismetSystemLibrary.PrintString` "Failed to create session"))))

(event `JoinSession`
  (params (Session :type "BlueprintSessionResult Structure"))
  (`JoinSessionCallbackProxy.JoinSession` (`GameplayStatics.GetPlayerController` 0) Session))

(event `self.HandleNetworkError`
  (params (FailureType :type "ENetworkFailure Enum" :default "NetDriverAlreadyExists") (bIsServer :type Boolean))
  (`KismetSystemLibrary.PrintString` (`KismetStringLibrary.Concat_StrStr` "Network Error! Failure:" (`|GetEnumeratorNameAsString` FailureType)) true true (struct :`R` 1.0 :`B` 0.105166 :`A` 1.0) 10.0)
  (`self.DestroySession`))

(event `LoadMap`
  (params (LevelName :type String))
  (bind _returnvalue (`GameplayStatics.GetPlayerController` 0))
  (`KismetSystemLibrary.ExecuteConsoleCommand` "servertravel DayNightTravel" _returnvalue)
  (`KismetSystemLibrary.Delay` 7.0)
  (`KismetSystemLibrary.ExecuteConsoleCommand` (`KismetStringLibrary.Concat_StrStr` "servertravel " LevelName) _returnvalue)
  (bind _asdrunk_game_mode (cast `/Game/Blueprints/GameMode/DrunkGameMode` (`GameplayStatics.GetGameMode`) :!label _label)
    (:`then`
      (`/Game/Blueprints/GameMode/DrunkGameMode.Countdown` _asdrunk_game_mode))
    (:`CastFailed`
      (`KismetSystemLibrary.PrintString` "Failed at casting to GameMode on GameInstance")
      (`KismetSystemLibrary.Delay` 0.2)
      (goto _label))))

(event `LoadFirstLevel`
  (`KismetSystemLibrary.ExecuteConsoleCommand` "servertravel Level0" (`GameplayStatics.GetPlayerController` 0)))

(event `PauseGame`
  (`GameplayStatics.SetGamePaused` true))

(event `UnpauseGame`
  (`GameplayStatics.SetGamePaused` false))

(event `LoadBack`
  (`KismetSystemLibrary.ExecuteConsoleCommand` "servertravel DrunkLobby?Game=/Game/Blueprints/GameMode/LobbyGameMode.LobbyGameMode" (`GameplayStatics.GetPlayerController` 0)))