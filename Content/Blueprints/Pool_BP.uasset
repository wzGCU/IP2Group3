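; Pool actor for a drunk-themed game that slows the player while inside its trigger volume.
; On overlap it sets the ThirdPersonCharacter's speed to 100, tells DrunkGameState the pool started and plays a splash-in sound at the pool; leaving restores speed to 400 and stops it.
; PoolShow and PoolClearMesh events toggle visibility by assigning or clearing the cube mesh and pool material.
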(event `PoolClearMesh`
  (bind _properpool (`self.ProperPool`))
  (`StaticMeshComponent.SetStaticMesh` _properpool null)
  (`PrimitiveComponent.SetMaterial` _properpool 0 null))

(event `PoolShow`
  (bind _properpool (`self.ProperPool`))
  (`StaticMeshComponent.SetStaticMesh` _properpool "/Game/Meshes/Default/1M_Cube.1M_Cube")
  (`PrimitiveComponent.SetMaterial` _properpool 0 "/Game/Materials/PoolMat.PoolMat"))

(event `self.TriggerVolume.OnComponentBeginOverlap`
  (params (OverlappedComponent :type "PrimitiveComponent Object Reference") (OtherActor :type "Actor Object Reference") (OtherComp :type "PrimitiveComponent Object Reference") (OtherBodyIndex :type Integer) (bFromSweep :type Boolean) (SweepResult :type "HitResult Structure (by ref)"))
  (bind _asthird_person_character (cast `/Game/Blueprints/ThirdPersonCharacter` OtherActor))
  (`/Game/Blueprints/ThirdPersonCharacter.Speed` _asthird_person_character 100.0)
  (bind _asdrunk_game_state (cast `/Game/Blueprints/GameMode/DrunkGameState` (`GameplayStatics.GetGameState`)))
  (`/Game/Blueprints/GameMode/DrunkGameState.PoolStart` _asdrunk_game_state)
  (`GameplayStatics.PlaySoundAtLocation` "/Game/Throwaways/Pool.Pool" (`SceneComponent.K2_GetComponentLocation` (`self.ProperPool`)) (struct) 1.0 1.0 0.0 null null null))

(event `self.TriggerVolume.OnComponentEndOverlap`
  (params (OverlappedComponent :type "PrimitiveComponent Object Reference") (OtherActor :type "Actor Object Reference") (OtherComp :type "PrimitiveComponent Object Reference") (OtherBodyIndex :type Integer))
  (bind _asthird_person_character (cast `/Game/Blueprints/ThirdPersonCharacter` OtherActor))
  (`/Game/Blueprints/ThirdPersonCharacter.Speed` _asthird_person_character 400.0)
  (bind _asdrunk_game_state (cast `/Game/Blueprints/GameMode/DrunkGameState` (`GameplayStatics.GetGameState`)))
  (`/Game/Blueprints/GameMode/DrunkGameState.PoolStop` _asdrunk_game_state))

(fn `UserConstructionScript`)