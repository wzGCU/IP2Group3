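; Yard Blueprint that swings four doors open when the ThirdPersonCharacter enters their trigger boxes.
; Each box overlap starts a fast looping timer that calls that door's opener event by name.
; The opener steps its anchor's relative yaw down in fixed increments and clears the timer once the open limit is reached.
; The logic is duplicated per door, and nothing closes them again.
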(event `Door1Opener`
  (bind _rdoor1anchor (`self.RDoor1Anchor`))
  (bind (_relativerotation_roll _relativerotation_pitch _relativerotation_yaw) (`KismetMathLibrary.BreakRotator` (`SceneComponent.RelativeRotation` _rdoor1anchor)))
  (`SceneComponent.K2_SetRelativeRotation` _rdoor1anchor (`KismetMathLibrary.MakeRotator` _relativerotation_roll _relativerotation_pitch (- _relativerotation_yaw 0.5)) false false)
  (if (<= _relativerotation_yaw -100.0)
    (`KismetSystemLibrary.K2_ClearAndInvalidateTimerHandle` (stale `self.Box.OnComponentBeginOverlap` _returnvalue))))

(event `self.Box.OnComponentBeginOverlap`
  (params (OverlappedComponent :type "PrimitiveComponent Object Reference") (OtherActor :type "Actor Object Reference") (OtherComp :type "PrimitiveComponent Object Reference") (OtherBodyIndex :type Integer) (bFromSweep :type Boolean) (SweepResult :type "HitResult Structure (by ref)"))
  (cast `/Game/Blueprints/ThirdPersonCharacter` OtherActor)
  (bind _returnvalue (`KismetSystemLibrary.K2_SetTimer` null "Door1Opener" 0.001 true)))

(event `Door2Opener`
  (bind _rdoor2anchor (`self.RDoor2Anchor`))
  (bind (_relativerotation_roll _relativerotation_pitch _relativerotation_yaw) (`KismetMathLibrary.BreakRotator` (`SceneComponent.RelativeRotation` _rdoor2anchor)))
  (`SceneComponent.K2_SetRelativeRotation` _rdoor2anchor (`KismetMathLibrary.MakeRotator` _relativerotation_roll _relativerotation_pitch (- _relativerotation_yaw 0.5)) false false)
  (if (<= _relativerotation_yaw -100.0)
    (`KismetSystemLibrary.K2_ClearAndInvalidateTimerHandle` (stale `self.Box1.OnComponentBeginOverlap` _returnvalue))))

(event `self.Box1.OnComponentBeginOverlap`
  (params (OverlappedComponent :type "PrimitiveComponent Object Reference") (OtherActor :type "Actor Object Reference") (OtherComp :type "PrimitiveComponent Object Reference") (OtherBodyIndex :type Integer) (bFromSweep :type Boolean) (SweepResult :type "HitResult Structure (by ref)"))
  (cast `/Game/Blueprints/ThirdPersonCharacter` OtherActor)
  (bind _returnvalue (`KismetSystemLibrary.K2_SetTimer` null "Door2Opener" 0.001 true)))

(event `Door3Opener`
  (bind _rdoor3anchor (`self.RDoor3Anchor`))
  (bind (_relativerotation_roll _relativerotation_pitch _relativerotation_yaw) (`KismetMathLibrary.BreakRotator` (`SceneComponent.RelativeRotation` _rdoor3anchor)))
  (`SceneComponent.K2_SetRelativeRotation` _rdoor3anchor (`KismetMathLibrary.MakeRotator` _relativerotation_roll _relativerotation_pitch (- _relativerotation_yaw 0.5)) false false)
  (if (<= _relativerotation_yaw -100.0)
    (`KismetSystemLibrary.K2_ClearAndInvalidateTimerHandle` (stale `self.Box2.OnComponentBeginOverlap` _returnvalue))))

(event `self.Box2.OnComponentBeginOverlap`
  (params (OverlappedComponent :type "PrimitiveComponent Object Reference") (OtherActor :type "Actor Object Reference") (OtherComp :type "PrimitiveComponent Object Reference") (OtherBodyIndex :type Integer) (bFromSweep :type Boolean) (SweepResult :type "HitResult Structure (by ref)"))
  (cast `/Game/Blueprints/ThirdPersonCharacter` OtherActor)
  (bind _returnvalue (`KismetSystemLibrary.K2_SetTimer` null "Door3Opener" 0.001 true)))

(event `Door4Opener`
  (bind _rdoor4anchor (`self.RDoor4Anchor`))
  (bind (_relativerotation_roll _relativerotation_pitch _relativerotation_yaw) (`KismetMathLibrary.BreakRotator` (`SceneComponent.RelativeRotation` _rdoor4anchor)))
  (`SceneComponent.K2_SetRelativeRotation` _rdoor4anchor (`KismetMathLibrary.MakeRotator` _relativerotation_roll _relativerotation_pitch (- _relativerotation_yaw 0.5)) false false)
  (if (<= _relativerotation_yaw -100.0)
    (`KismetSystemLibrary.K2_ClearAndInvalidateTimerHandle` (stale `self.Box3.OnComponentBeginOverlap` _returnvalue))))

(event `self.Box3.OnComponentBeginOverlap`
  (params (OverlappedComponent :type "PrimitiveComponent Object Reference") (OtherActor :type "Actor Object Reference") (OtherComp :type "PrimitiveComponent Object Reference") (OtherBodyIndex :type Integer) (bFromSweep :type Boolean) (SweepResult :type "HitResult Structure (by ref)"))
  (cast `/Game/Blueprints/ThirdPersonCharacter` OtherActor)
  (bind _returnvalue (`KismetSystemLibrary.K2_SetTimer` null "Door4Opener" 0.001 true)))

(fn `UserConstructionScript`)