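; Beer pickup actor that lowers the DrunkGameState's current game time when the ThirdPersonCharacter touches it.
; The first valid overlap subtracts the time behind a DoOnce and plays a pickup sound at the mesh.
; A looping timer then calls BeerSmallizer to shrink the actor for a second before it is destroyed.
; Separate BeerShow and BeerClearMesh events set or clear the beer's static mesh.
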(event `BeerClearMesh`
  (`StaticMeshComponent.SetStaticMesh` (`self.BeerMesh`) null))

(event `BeerShow`
  (`StaticMeshComponent.SetStaticMesh` (`self.BeerMesh`) "/Game/Meshes/Placeholders/Beer.Beer"))

(event `BeerSmallizer`
  (bind (_returnvalue_x _returnvalue_y _returnvalue_z) (`KismetMathLibrary.BreakVector` (`self.GetActorScale3D`)))
  (`self.SetActorScale3D` (`KismetMathLibrary.MakeVector` (- _returnvalue_x 0.01) (- _returnvalue_y 0.01) (- _returnvalue_z 0.01))))

(event `self.ReceiveActorBeginOverlap`
  (params (OtherActor :type "Actor Object Reference"))
  (if (== (`GameplayStatics.GetObjectClass` OtherActor) "/Game/Blueprints/ThirdPersonCharacter.ThirdPersonCharacter_C")
    (bind _asdrunk_game_state (cast `/Game/Blueprints/GameMode/DrunkGameState` (`GameplayStatics.GetGameState`)))
    (`/Engine/EditorBlueprintResources/StandardMacros.DoOnce` false
      (:`Completed`
        (set `/Game/Blueprints/GameMode/DrunkGameState.Game_CurrentTime` (- (`/Game/Blueprints/GameMode/DrunkGameState.Game_CurrentTime` _asdrunk_game_state) 20.0) _asdrunk_game_state)
        (`GameplayStatics.PlaySoundAtLocation` "/Game/Throwaways/FlowerTaken.FlowerTaken" (`SceneComponent.K2_GetComponentLocation` (`self.BeerMesh`)) (struct) 1.0 1.0 0.0 null null null)
        (bind _returnvalue (`KismetSystemLibrary.K2_SetTimer` null "BeerSmallizer" 0.01 true))
        (`KismetSystemLibrary.Delay` 1.0)
        (`KismetSystemLibrary.K2_ClearAndInvalidateTimerHandle` _returnvalue)
        (`self.K2_DestroyActor`)))))

(fn `UserConstructionScript`)