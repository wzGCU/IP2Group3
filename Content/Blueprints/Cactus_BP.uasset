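; Cactus obstacle that launches, stuns and plays a hit sound on any ThirdPersonCharacter overlapping its capsule, then adds to the DrunkGameState noise.
; On BeginPlay it polls until the game state reports BothIn, with a delayed fallback if that cast fails.
; The authority rolls RandomAssign, which picks a P1Vis or P2Vis tag alongside VisibilityBased.
; CactusTrueMesh and CactusFakeMesh events swap the mesh between cactus and flower.
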(event `CactusTrueMesh`
  (`StaticMeshComponent.SetStaticMesh` (`self.CactiMesh`) "/Game/Meshes/ObstaclesNCollectibles/C12_Cactus.C12_Cactus"))

(event `CactusFakeMesh`
  (`StaticMeshComponent.SetStaticMesh` (`self.CactiMesh`) "/Game/Meshes/ObstaclesNCollectibles/C12_Flower.C12_Flower"))

(event `self.Capsule.OnComponentBeginOverlap`
  (params (OverlappedComponent :type "PrimitiveComponent Object Reference") (OtherActor :type "Actor Object Reference") (OtherComp :type "PrimitiveComponent Object Reference") (OtherBodyIndex :type Integer) (bFromSweep :type Boolean) (SweepResult :type "HitResult Structure (by ref)"))
  (bind _asthird_person_character (cast `/Game/Blueprints/ThirdPersonCharacter` OtherActor))
  (`/Engine/EditorBlueprintResources/StandardMacros.DoOnce` false :!label _label
    (:`Completed`
      (bind (_returnvalue_x _returnvalue_y) (`KismetMathLibrary.BreakVector` (`self.GetVelocity` _asthird_person_character)))
      (`Character.LaunchCharacter` _asthird_person_character (`KismetMathLibrary.MakeVector` -1000.0 (* _returnvalue_y -1.5)) false false)
      (`/Game/Blueprints/ThirdPersonCharacter.StunCharacter` _asthird_person_character 2.0)
      (`GameplayStatics.PlaySoundAtLocation` "/Game/Audios/ObstacleHit.ObstacleHit" (`SceneComponent.K2_GetComponentLocation` (`self.CactiMesh`)) (struct) 1.0 1.0 0.0 null null null)
      (bind _asdrunk_game_state (cast `/Game/Blueprints/GameMode/DrunkGameState` (`GameplayStatics.GetGameState`)))
      (`/Game/Blueprints/GameMode/DrunkGameState.AddToNoise` _asdrunk_game_state 0.1)
      (goto _label :!via `Reset`))))

(event `self.ReceiveBeginPlay`
  (bind _returnvalue (`ActorComponent.GetOwner` (`self.StaticMeshComponent`)))
  (`KismetSystemLibrary.Delay` 1.0 :!label _label_2)
  (bind _asdrunk_game_state (cast `/Game/Blueprints/GameMode/DrunkGameState` (`GameplayStatics.GetGameState`))
    (:`then`
      (if (`/Game/Blueprints/GameMode/DrunkGameState.BothIn` _asdrunk_game_state)
        _
        (else
          (goto _label_2))))
    (:`CastFailed`
      (`KismetSystemLibrary.Delay` 5.0)))
  (`/Engine/EditorBlueprintResources/ActorMacros.Switch Has Authority`
    (:`Authority`
      (set `self.RandomAssign` (`KismetMathLibrary.RandomFloatInRange` 0.0 100.0)))
    (:`Remote`
      (`KismetSystemLibrary.Delay` 0.2)))
  (if (> (`self.RandomAssign`) 50.0)
    (set `Actor.Tags` (`|MakeArray` "VisibilityBased" "P1Vis" :!type "Name") _returnvalue)
    (else
      (set `Actor.Tags` (`|MakeArray` "VisibilityBased" "P2Vis" :!type "Name") _returnvalue))))

(fn `UserConstructionScript`)