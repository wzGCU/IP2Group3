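; DrunkGameMode is a game mode that handles player logins for a multiplayer game.
; On PostLogin it casts the new player to DrunkGameController, calls ClientDrawHUD on it and adds it to PlayerControllers.
; Once two or more controllers are stored, it prints a debug string and calls PlayersArray on DrunkGameState, repeating this for each later login.
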(event `self.K2_PostLogin`
  (params (NewPlayer :type "PlayerController Object Reference"))
  (bind _asdrunk_game_controller (cast `/Game/Blueprints/DrunkGameController` NewPlayer))
  (`/Game/Blueprints/DrunkGameController.Client_DrawHUD` _asdrunk_game_controller)
  (`KismetArrayLibrary.Array_Add` (`self.PlayerControllers`) NewPlayer)
  (if (>= (`KismetArrayLibrary.Array_Length` (`self.PlayerControllers`)) 2)
    (`KismetSystemLibrary.PrintString` "tru")
    (bind _asdrunk_game_state (cast `/Game/Blueprints/DrunkGameState` (`GameplayStatics.GetGameState`)))
    (`/Game/Blueprints/DrunkGameState.PlayersArray` _asdrunk_game_state)))

(fn `UserConstructionScript`)