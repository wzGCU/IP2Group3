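; LobbyGameMode is the lobby game mode that tracks connected player controllers and keeps each client's player list in sync.
; Joins render the lobby widget on the new client, and joins and logouts both trigger UpdateServer.
; UpdateServer clears and refills every client's list with names and Steam avatars, retrying failed avatar fetches and delaying those still loading.
; KickPlayer kicks the DrunkGameController at a given index.
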(event `self.K2_PostLogin`
  (params (NewPlayer :type "PlayerController Object Reference"))
  (`KismetArrayLibrary.Array_Add` (`self.PlayerControllers`) NewPlayer)
  (bind _asdrunk_game_controller (cast `/Game/Blueprints/GameMode/DrunkGameController` NewPlayer))
  (`/Game/Blueprints/GameMode/DrunkGameController.Client_RenderLobbyW` _asdrunk_game_controller)
  (`self.UpdateServer`))

(event `self.K2_OnLogout`
  (params (ExitingController :type "Controller Object Reference"))
  (bind _playercontrollers (`self.PlayerControllers`))
  (for (_array_element _array_index) _playercontrollers
    (if (== ExitingController _array_element)
      (break)))
  (`KismetArrayLibrary.Array_Remove` _playercontrollers _array_index)
  (`self.UpdateServer`))

(event `UpdateServer`
  (for _array_element (`self.PlayerControllers`)
    (bind _asdrunk_game_controller (cast `/Game/Blueprints/GameMode/DrunkGameController` _array_element))
    (`/Game/Blueprints/GameMode/DrunkGameController.Client_ClearPL` _asdrunk_game_controller)
    (for (_array_element_2 _array_index) (`self.PlayerControllers`)
      (bind _returnvalue (`AdvancedSteamFriendsLibrary.GetSteamFriendAvatar` (`AdvancedSessionsLibrary.GetUniqueNetID` _array_element_2) :!label _label)
        (:`OnSuccess`
          _)
        (:`AsyncLoading`
          (`KismetSystemLibrary.PrintString` "Async loading..")
          (`KismetSystemLibrary.Delay` 2.0))
        (:`OnFailure`
          (`KismetSystemLibrary.Delay` 1.0)
          (goto _label)))
      (`/Game/Blueprints/GameMode/DrunkGameController.AddPlayer` _asdrunk_game_controller false (`KismetTextLibrary.Conv_StringToText` (`AdvancedSessionsLibrary.GetPlayerName` _array_element_2)) _returnvalue _array_index))))

(event `KickPlayer`
  (params (Index :type Integer))
  (bind _asdrunk_game_controller (cast `/Game/Blueprints/GameMode/DrunkGameController` (`|GetArrayItem` (`self.PlayerControllers`) Index)))
  (`/Game/Blueprints/GameMode/DrunkGameController.Kick` _asdrunk_game_controller))

(fn `UserConstructionScript`)