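; Lobby controller that manages a player's lobby UI and handles being kicked from a session.
; Client-prefixed events create and show the Lobby_W widget, remove it, or clear its player list.
; AddPlayer forwards player, avatar, index and fail data to that stored widget to build the list.
; Kick opens the main menu, prints a notice that the host kicked the player, and destroys the session.
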(event `Client_RenderLobbyW`
  (bind _returnvalue (`|CreateWidget` "/Game/MainMenu/Lobby_W.Lobby_W_C"))
  (bind _output_get (set `self.Lobby Widget` _returnvalue))
  (`UserWidget.AddToViewport` _output_get 1))

(event `Client_RemoveLobbyW`
  (`Widget.RemoveFromParent` (`self.Lobby Widget`)))

(event `AddPlayer`
  (params (`Fail?` :type Boolean) (Player :type Text) (Avatar :type "Texture2D Object Reference") (PlayerIndex :type Integer))
  (`/Game/MainMenu/Lobby_W.AddPlayerToList` (`self.Lobby Widget`) `Fail?` Player Avatar PlayerIndex))

(event `Client_ClearPL`
  (`/Game/MainMenu/Lobby_W.ClearPlayersList` (`self.Lobby Widget`)))

(event `Kick`
  (`GameplayStatics.OpenLevelBySoftObjectPtr` "/Game/Maps/MainMenu.MainMenu")
  (`KismetSystemLibrary.PrintString` "You were kicked from the session by host." true true (struct :`R` 1.0 :`B` 0.029831 :`A` 1.0) 10.0)
  (`DestroySessionCallbackProxy.DestroySession` self))

(fn `UserConstructionScript`)