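; Player controller for a two-player online game, handling per-client UI, camera and input.
; Client events drive lobby, connecting, cinematic, level start, countdown, HUD, completion and game-over screens, plus host kicks back to the main menu.
; Camera events switch each player to their own DrunkCamera.
; Render events create asymmetric views by clearing obstacle meshes tagged for the other player and swapping cacti between true and fake meshes.
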(event `Client_RenderOnAnotherNight`
  (bind _returnvalue (`|CreateWidget` "/Game/UI/Widgets/W_OnAnotherNight.W_OnAnotherNight_C"))
  (`UserWidget.AddToViewport` _returnvalue 0)
  (`KismetSystemLibrary.Delay` 6.0)
  (`self.Client_RenderConnectingWidget`))

(event `Client_RenderConnectingWidget`
  (bind _returnvalue (`|CreateWidget` "/Game/UI/Widgets/W_Connecting.W_Connecting_C"))
  (bind _output_get (set `self.ConnectingWidgetRef` _returnvalue))
  (`UserWidget.AddToViewport` _output_get 0))

(event `Client_DestroyConnectingWidget`
  (`Widget.RemoveFromParent` (`self.ConnectingWidgetRef`)))

(event `Client_StartCinematic`
  (bind _returnvalue (`|CreateWidget` "/Game/UI/Widgets/Todo/Cinematic.Cinematic_C"))
  (bind _output_get (set `self.CinematicReference` _returnvalue))
  (`UserWidget.AddToViewport` _output_get 0))

(event `Client_DeleteCinematic`
  (`Widget.RemoveFromParent` (`self.CinematicReference`)))

(event `Client_RenderLobbyW`
  (bind _returnvalue (`|CreateWidget` "/Game/UI/Widgets/Lobby_W.Lobby_W_C"))
  (bind _output_get (set `self.Lobby Widget` _returnvalue))
  (`UserWidget.AddToViewport` _output_get 1))

(event `Client_RemoveLobbyW`
  (`Widget.RemoveFromParent` (`self.Lobby Widget`)))

(event `AddPlayer`
  (params (`Fail?` :type Boolean) (Player :type Text) (Avatar :type "Texture2D Object Reference") (PlayerIndex :type Integer))
  (`/Game/UI/Widgets/Lobby_W.AddPlayerToList` (`self.Lobby Widget`) `Fail?` Player Avatar PlayerIndex))

(event `Client_ClearPL`
  (`/Game/UI/Widgets/Lobby_W.ClearPlayersList` (`self.Lobby Widget`)))

(event `Kick`
  (`GameplayStatics.OpenLevelBySoftObjectPtr` "/Game/Maps/MainMenu.MainMenu")
  (`KismetSystemLibrary.PrintString` "You were kicked from the session by host." true true (struct :`R` 1.0 :`B` 0.029831 :`A` 1.0) 10.0)
  (`DestroySessionCallbackProxy.DestroySession` self))

(event `Input_Game`
  (`WidgetBlueprintLibrary.SetInputMode_GameOnly` self))

(event `Input_UI`
  (`WidgetBlueprintLibrary.SetInputMode_UIOnlyEx` self null))

(event `Client_GameCompleted`
  (bind _returnvalue (`|CreateWidget` "/Game/UI/Widgets/W_LastLevelCompleted.W_LastLevelCompleted_C"))
  (`UserWidget.AddToViewport` _returnvalue 0))

(event `Input_GameUI`
  (`WidgetBlueprintLibrary.SetInputMode_GameAndUIEx` self null))

(event `Client_Camera1`
  ;[1 1 1] Rendering Cameras
  (bind _returnvalue (`GameplayStatics.GetActorOfClass` "/Game/Blueprints/DrunkCameraP1.DrunkCameraP1_C"))
  (`self.SetViewTargetWithBlend` _returnvalue))

(event `Client_Camera2`
  ;[1 1 1] Rendering Cameras
  (bind _returnvalue (`GameplayStatics.GetActorOfClass` "/Game/Blueprints/DrunkCameraP2.DrunkCameraP2_C"))
  (`self.SetViewTargetWithBlend` _returnvalue))

(event `Client_OnLevelStart`
  (`self.Client_DestroyConnectingWidget`)
  (`self.Input_GameUI`)
  (bind _returnvalue (`|CreateWidget` "/Game/UI/Widgets/W_OnLevel.W_OnLevel_C"))
  (bind _output_get (set `self.StartWidgetReference` _returnvalue))
  (`UserWidget.AddToViewport` _output_get 2))

(event `Client_ShowCountdown`
  (`Widget.RemoveFromParent` (`self.StartWidgetReference`))
  (`self.Input_Game`)
  (bind _returnvalue (`|CreateWidget` "/Game/UI/Widgets/W_Countdown.W_Countdown_C"))
  (`UserWidget.AddToViewport` _returnvalue 3)
  (`KismetSystemLibrary.Delay` 4.0)
  (bind _returnvalue_2 (`|CreateWidget` "/Game/UI/Widgets/W_HUD.W_HUD_C"))
  (bind _output_get (set `self.HUDWidgetReference` _returnvalue_2))
  (`UserWidget.AddToViewport` _output_get 4))

(event `Server_LevelComplete`
  (`Widget.RemoveFromParent` (`self.HUDWidgetReference`))
  (bind _returnvalue (`|CreateWidget` "/Game/UI/Widgets/W_LevelCompleted.W_LevelCompleted_C"))
  (`UserWidget.AddToViewport` _returnvalue 5))

(event `Server_GameOver`
  ;[1 0.00954 0.04934] GameOver Handler
  (bind _returnvalue (`|CreateWidget` "/Game/UI/Widgets/W_GameOver.W_GameOver_C"))
  (`UserWidget.AddToViewport` _returnvalue 5)
  (`GameplayStatics.PlaySound2D` "/Game/Audios/Cues/C_GameOver.C_GameOver" 1.0 1.0 0.0 null null)
  (set `self.bShowMouseCursor` true)
  (`self.Input_UI`)
  (`KismetSystemLibrary.Delay` 5.0)
  (`Widget.RemoveFromParent` _returnvalue)
  (`Widget.RemoveFromParent` (`self.HUDWidgetReference`))
  (`self.Client_RenderLobbyW`))

(event `Client_RenderObjectsPlayer2`
  ;[1 0 0.7088] Deleting meshes for each player mechanic
  (bind _outactors (`GameplayStatics.GetAllActorsOfClassWithTag` "/Game/Blueprints/TrashCan_BP.TrashCan_BP_C" "P1Vis"))
  (for _array_element _outactors
    (`/Game/Blueprints/TrashCan_BP.TrashClearMesh` _array_element))
  (bind _outactors_2 (`GameplayStatics.GetAllActorsOfClassWithTag` "/Game/Blueprints/Beer_BP.Beer_BP_C" "P1Vis"))
  (for _array_element_2 _outactors_2
    (`/Game/Blueprints/Beer_BP.BeerClearMesh` _array_element_2))
  (bind _outactors_3 (`GameplayStatics.GetAllActorsOfClassWithTag` "/Game/Blueprints/Cactus_BP.Cactus_BP_C" "P1Vis"))
  (for _array_element_3 _outactors_3
    (`/Game/Blueprints/Cactus_BP.CactusFakeMesh` _array_element_3))
  (bind _outactors_4 (`GameplayStatics.GetAllActorsOfClassWithTag` "/Game/Blueprints/Cactus_BP.Cactus_BP_C" "P2Vis"))
  (for _array_element_4 _outactors_4
    (`/Game/Blueprints/Cactus_BP.CactusTrueMesh` _array_element_4))
  (bind _outactors_5 (`GameplayStatics.GetAllActorsOfClassWithTag` "/Game/Blueprints/Flower_BP.Flower_BP_C" "P1Vis"))
  (for _array_element_5 _outactors_5
    (`/Game/Blueprints/Flower_BP.FlowerClearMesh` _array_element_5))
  (bind _outactors_6 (`GameplayStatics.GetAllActorsOfClassWithTag` "/Game/Blueprints/Pool_BP2.Pool_BP2_C" "P1Vis"))
  (for _array_element_6 _outactors_6
    (`/Game/Blueprints/Pool_BP2.PoolClearMesh` _array_element_6))
  (bind _outactors_7 (`GameplayStatics.GetAllActorsOfClassWithTag` "/Game/Blueprints/SkateboardDown_BP.SkateboardDown_BP_C" "P1Vis"))
  (for _array_element_7 _outactors_7
    (`/Game/Blueprints/SkateboardDown_BP.SkateboardDownClearMesh` _array_element_7))
  (bind _outactors_8 (`GameplayStatics.GetAllActorsOfClassWithTag` "/Game/Blueprints/SkateboardLeft_BP.SkateboardLeft_BP_C" "P1Vis"))
  (for _array_element_8 _outactors_8
    (`/Game/Blueprints/SkateboardLeft_BP.SkateboardLeftClearMesh` _array_element_8))
  (bind _outactors_9 (`GameplayStatics.GetAllActorsOfClassWithTag` "/Game/Blueprints/SkateboardRight_BP.SkateboardRight_BP_C" "P1Vis"))
  (for _array_element_9 _outactors_9
    (`/Game/Blueprints/SkateboardRight_BP.SkateboardRightClearMesh` _array_element_9))
  (bind _outactors_10 (`GameplayStatics.GetAllActorsOfClassWithTag` "/Game/Blueprints/SkateboardUp_BP.SkateboardUp_BP_C" "P1Vis"))
  (for _array_element_10 _outactors_10
    (`/Game/Blueprints/SkateboardUp_BP.SkateboardUpClearMesh` _array_element_10))
  (bind _outactors_11 (`GameplayStatics.GetAllActorsOfClassWithTag` "/Game/Blueprints/Trampoline_BP.Trampoline_BP_C" "P1Vis"))
  (for _array_element_11 _outactors_11
    (`/Game/Blueprints/Trampoline_BP.TrampolineClearMesh` _array_element_11))
  (bind _outactors_12 (`GameplayStatics.GetAllActorsOfClassWithTag` "/Game/Blueprints/WaterSprinkler_BP.WaterSprinkler_BP_C" "P1Vis"))
  (for _array_element_12 _outactors_12
    (`/Game/Blueprints/WaterSprinkler_BP.SprinklerClearMesh` _array_element_12)))

(event `Client_RenderObjectsPlayer1`
  ;[1 0 0.7088] Deleting meshes for each player mechanic
  (bind _outactors (`GameplayStatics.GetAllActorsOfClassWithTag` "/Game/Blueprints/TrashCan_BP.TrashCan_BP_C" "P2Vis"))
  (for _array_element _outactors
    (`/Game/Blueprints/TrashCan_BP.TrashClearMesh` _array_element))
  (bind _outactors_2 (`GameplayStatics.GetAllActorsOfClassWithTag` "/Game/Blueprints/Beer_BP.Beer_BP_C" "P2Vis"))
  (for _array_element_2 _outactors_2
    (`/Game/Blueprints/Beer_BP.BeerClearMesh` _array_element_2))
  (bind _outactors_3 (`GameplayStatics.GetAllActorsOfClassWithTag` "/Game/Blueprints/Cactus_BP.Cactus_BP_C" "P2Vis"))
  (for _array_element_3 _outactors_3
    (`/Game/Blueprints/Cactus_BP.CactusFakeMesh` _array_element_3))
  (bind _outactors_4 (`GameplayStatics.GetAllActorsOfClassWithTag` "/Game/Blueprints/Cactus_BP.Cactus_BP_C" "P1Vis"))
  (for _array_element_4 _outactors_4
    (`/Game/Blueprints/Cactus_BP.CactusTrueMesh` _array_element_4))
  (bind _outactors_5 (`GameplayStatics.GetAllActorsOfClassWithTag` "/Game/Blueprints/Flower_BP.Flower_BP_C" "P2Vis"))
  (for _array_element_5 _outactors_5
    (`/Game/Blueprints/Flower_BP.FlowerClearMesh` _array_element_5))
  (bind _outactors_6 (`GameplayStatics.GetAllActorsOfClassWithTag` "/Game/Blueprints/Pool_BP2.Pool_BP2_C" "P2Vis"))
  (for _array_element_6 _outactors_6
    (`/Game/Blueprints/Pool_BP2.PoolClearMesh` _array_element_6))
  (bind _outactors_7 (`GameplayStatics.GetAllActorsOfClassWithTag` "/Game/Blueprints/SkateboardDown_BP.SkateboardDown_BP_C" "P2Vis"))
  (for _array_element_7 _outactors_7
    (`/Game/Blueprints/SkateboardDown_BP.SkateboardDownClearMesh` _array_element_7))
  (bind _outactors_8 (`GameplayStatics.GetAllActorsOfClassWithTag` "/Game/Blueprints/SkateboardLeft_BP.SkateboardLeft_BP_C" "P2Vis"))
  (for _array_element_8 _outactors_8
    (`/Game/Blueprints/SkateboardLeft_BP.SkateboardLeftClearMesh` _array_element_8))
  (bind _outactors_9 (`GameplayStatics.GetAllActorsOfClassWithTag` "/Game/Blueprints/SkateboardRight_BP.SkateboardRight_BP_C" "P2Vis"))
  (for _array_element_9 _outactors_9
    (`/Game/Blueprints/SkateboardRight_BP.SkateboardRightClearMesh` _array_element_9))
  (bind _outactors_10 (`GameplayStatics.GetAllActorsOfClassWithTag` "/Game/Blueprints/SkateboardUp_BP.SkateboardUp_BP_C" "P2Vis"))
  (for _array_element_10 _outactors_10
    (`/Game/Blueprints/SkateboardUp_BP.SkateboardUpClearMesh` _array_element_10))
  (bind _outactors_11 (`GameplayStatics.GetAllActorsOfClassWithTag` "/Game/Blueprints/Trampoline_BP.Trampoline_BP_C" "P2Vis"))
  (for _array_element_11 _outactors_11
    (`/Game/Blueprints/Trampoline_BP.TrampolineClearMesh` _array_element_11))
  (bind _outactors_12 (`GameplayStatics.GetAllActorsOfClassWithTag` "/Game/Blueprints/WaterSprinkler_BP.WaterSprinkler_BP_C" "P2Vis"))
  (for _array_element_12 _outactors_12
    (`/Game/Blueprints/WaterSprinkler_BP.SprinklerClearMesh` _array_element_12)))

(fn `UserConstructionScript`)