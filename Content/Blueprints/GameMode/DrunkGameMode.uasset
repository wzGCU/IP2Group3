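; Game mode for a two-player co-op level that waits for both players, runs the countdown and decides success or failure.
; PostLogin triggers the countdown, which shuffles "VisibilityBased" actors into the game instance, has each client render its objects and starts the timer.
; Tick polls DrunkGameState, ending the game on excess noise, timeout or too few flowers at the finish.
; With enough flowers, it completes the level and loads the next map.
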(event `random`
  (bind _outactors (`GameplayStatics.GetAllActorsWithTag` "VisibilityBased"))
  (`KismetArrayLibrary.Array_Shuffle` _outactors)
  (bind _output_get (set `self.VisibilityActors` _outactors))
  (bind _asdrunk_game_instance (cast `/Game/Blueprints/DrunkGameInstance` (`GameplayStatics.GetGameInstance`)))
  (`/Game/Blueprints/DrunkGameInstance.AssignObjects` _asdrunk_game_instance _output_get))

(event `GameOver`
  (params (InString :type String))
  (`KismetSystemLibrary.PrintString` InString true true (struct :`R` 1.0 :`G` 0.134509 :`B` 0.118592 :`A` 1.0) 5.0)
  (for _array_element (`self.PlayerControllers`)
    (bind _asdrunk_game_controller (cast `/Game/Blueprints/GameMode/DrunkGameController` _array_element))
    (`/Game/Blueprints/GameMode/DrunkGameController.Server_GameOver` _asdrunk_game_controller))
  (for _array_element_2 (`self.PlayerCharacters`)
    (`/Game/Blueprints/ThirdPersonCharacter.DisableMovement` _array_element_2))
  (bind _asdrunk_game_instance (cast `/Game/Blueprints/DrunkGameInstance` (`GameplayStatics.GetGameInstance`)))
  (`/Game/Blueprints/DrunkGameInstance.PauseGame` _asdrunk_game_instance))

(event `Countdown`
  (bind _returnvalue (`GameplayStatics.GetGameState`))
  (bind _asdrunk_game_state (cast `/Game/Blueprints/GameMode/DrunkGameState` (`GameplayStatics.GetGameState`)))
  (set `/Game/Blueprints/GameMode/DrunkGameState.TimerRunning` false _asdrunk_game_state)
  (bind _outactors (`GameplayStatics.GetAllActorsOfClass` "/Game/Blueprints/ThirdPersonCharacter.ThirdPersonCharacter_C"))
  (for _array_element _outactors
    (`/Game/Blueprints/ThirdPersonCharacter.StartCountDown` _array_element)
    (`self.random`))
  (for _array_element_2 (`self.PlayerControllers`)
    (bind _asdrunk_game_controller (cast `/Game/Blueprints/GameMode/DrunkGameController` _array_element_2))
    (`/Game/Blueprints/GameMode/DrunkGameController.Client_ShowCountdown` _asdrunk_game_controller))
  (`|ExecutionSequence`
    (:`then_0`
      (`self.RenderMeshesOnLevel`))
    (:`then_1`
      (`KismetSystemLibrary.Delay` 3.9)
      (bind _asdrunk_game_state_2 (cast `/Game/Blueprints/GameMode/DrunkGameState` _returnvalue))
      (set `/Game/Blueprints/GameMode/DrunkGameState.TimerRunning` true _asdrunk_game_state_2)
      (bind _asdrunk_game_instance (cast `/Game/Blueprints/DrunkGameInstance` (`GameplayStatics.GetGameInstance`)))
      (`/Game/Blueprints/DrunkGameInstance.UnpauseGame` _asdrunk_game_instance))
    (:`then_2`
      (bind _asdrunk_game_state_3 (cast `/Game/Blueprints/GameMode/DrunkGameState` _returnvalue))
      (`/Game/Blueprints/GameMode/DrunkGameState.PlayersArray` _asdrunk_game_state_3))))

(event `RenderMeshesOnLevel`
  (`|ExecutionSequence`
    (:`then_0`
      (bind _asdrunk_game_controller (cast `/Game/Blueprints/GameMode/DrunkGameController` (`|GetArrayItem` (`self.PlayerControllers`))))
      (`KismetSystemLibrary.Delay` 1.0)
      (`/Game/Blueprints/GameMode/DrunkGameController.Client_RenderObjectsPlayer1` _asdrunk_game_controller))
    (:`then_1`
      (bind _asdrunk_game_controller_2 (cast `/Game/Blueprints/GameMode/DrunkGameController` (`|GetArrayItem` (`self.PlayerControllers`) 1)))
      (`KismetSystemLibrary.Delay` 1.0)
      (`/Game/Blueprints/GameMode/DrunkGameController.Client_RenderObjectsPlayer2` _asdrunk_game_controller_2))))

(event `self.K2_PostLogin`
  (params (NewPlayer :type "PlayerController Object Reference"))
  ;[1 0.2851 0.2154] Draw HUD and add Player Controller Reference and send this over to Game State if there are two players.
  (`KismetArrayLibrary.Array_Add` (`self.PlayerControllers`) NewPlayer)
  (if (>= (`KismetArrayLibrary.Array_Length` (`self.PlayerControllers`)) 2)
    (`KismetSystemLibrary.Delay` 1.0)
    (bind _outactors (`GameplayStatics.GetAllActorsOfClass` "/Game/Blueprints/ThirdPersonCharacter.ThirdPersonCharacter_C"))
    (set `self.PlayerCharacters` _outactors)
    (`self.Countdown`)
    (else
      (`KismetSystemLibrary.PrintString` "Wait for 2nd player..."))))

(event `self.ReceiveTick`
  (params (DeltaSeconds :type "Float (single-precision)"))
  (if (`self.GameIsOn`)
    (`|ExecutionSequence`
      (:`then_0`
        ;[0.02376 0 1] Check if Noise Level is >= 100%
        (bind _asdrunk_game_state (cast `/Game/Blueprints/GameMode/DrunkGameState` (`GameplayStatics.GetGameState`)))
        (if (>= (`/Game/Blueprints/GameMode/DrunkGameState.NoiseCurrentValue` _asdrunk_game_state) 1.0)
          (`self.GameOver` "You made too much noise!")))
      (:`then_1`
        ;[1 0 0.0864] Check if Time has passed
        (bind _asdrunk_game_state_2 (cast `/Game/Blueprints/GameMode/DrunkGameState` (`GameplayStatics.GetGameState`)))
        (if (>= (`/Game/Blueprints/GameMode/DrunkGameState.Game_CurrentTime` _asdrunk_game_state_2) (`/Game/Blueprints/GameMode/DrunkGameState.Game_MaximumTime` _asdrunk_game_state_2))
          (`self.GameOver` "You run out of time!")))
      (:`then_2`
        (bind _asdrunk_game_state_3 (cast `/Game/Blueprints/GameMode/DrunkGameState` (`GameplayStatics.GetGameState`)))
        (if (`/Game/Blueprints/GameMode/DrunkGameState.LevelFinished` _asdrunk_game_state_3)
          (if (not (`self.DidOnce`))
            (set `self.DidOnce` true)
            (bind _asdrunk_game_state_4 (cast `/Game/Blueprints/GameMode/DrunkGameState` (`GameplayStatics.GetGameState`)))
            (if (>= (`/Game/Blueprints/GameMode/DrunkGameState.Game_FlowersCollected` _asdrunk_game_state_4) (`/Game/Blueprints/GameMode/DrunkGameState.Game_MaximumFlowers` _asdrunk_game_state_4))
              (for _array_element (`self.PlayerControllers`)
                (bind _asdrunk_game_controller (cast `/Game/Blueprints/GameMode/DrunkGameController` _array_element))
                (`/Game/Blueprints/GameMode/DrunkGameController.Server_LevelComplete` _asdrunk_game_controller)
                (`KismetSystemLibrary.Delay` 5.0)
                (for _array_element_2 (`self.PlayerCharacters`)
                  (`/Game/Blueprints/ThirdPersonCharacter.PreparingForNext` _array_element_2))
                (bind _asdrunk_game_state_5 (cast `/Game/Blueprints/GameMode/DrunkGameState` (`GameplayStatics.GetGameState`)))
                (set `/Game/Blueprints/GameMode/DrunkGameState.LevelFinished` false _asdrunk_game_state_5)
                (bind _asdrunk_game_instance (cast `/Game/Blueprints/DrunkGameInstance` (`GameplayStatics.GetGameInstance`))
                  (:`then`
                    (`/Game/Blueprints/DrunkGameInstance.LoadMap` _asdrunk_game_instance (`/Game/Blueprints/GameMode/DrunkGameState.NextLevelName` _asdrunk_game_state_5))
                    (set `self.DidOnce` false))
                  (:`CastFailed`
                    (`KismetSystemLibrary.PrintString` "Failed at casting at the end of the level"))))
              (else
                (`self.GameOver` "You did not collect enough flowers!")))))))))

(fn `UserConstructionScript`)