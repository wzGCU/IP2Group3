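; Game state for a two-player level, tracking shared noise, elapsed time, each player's X progress for UI and level completion.
; Looping timers decay noise and advance the clock while it runs; pool and sprinkler start/stop events toggle noise-adding timers, and AddToNoise adds arbitrary amounts.
; PlayersArray caches both characters after short delays, enabling Tick to read positions and briefly pulse LevelFinished when both touch the finish.
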(event `self.ReceiveBeginPlay`
  (bind _returnvalue (`KismetSystemLibrary.K2_SetTimer` null "NoiseDecreaser" 0.01 true))
  (bind _returnvalue_2 (`KismetSystemLibrary.K2_SetTimer` null "TimeIncreaser" 0.02 true)))

(event `self.ReceiveTick`
  (params (DeltaSeconds :type "Float (single-precision)"))
  (bind _output (`|GetArrayItem` (`self.Characters`)))
  (bind _output_2 (`|GetArrayItem` (`self.Characters`) 1))
  (bind _returnvalue_x (`KismetMathLibrary.BreakVector` (`SceneComponent.K2_GetComponentLocation` (`Actor.RootComponent` _output_2))))
  (bind _returnvalue_x_2 (`KismetMathLibrary.BreakVector` (`SceneComponent.K2_GetComponentLocation` (`Actor.RootComponent` _output))))
  (if (`self.CompletedSearch`)
    (`|ExecutionSequence`
      (:`then_0`
        ;[0.4199 1 0.3517] Getting Players Location (for UI)
        (`|ExecutionSequence`
          (:`then_0`
            (set `self.PlayerOneProgress` _returnvalue_x_2))
          (:`then_1`
            (set `self.PlayerTwoProgress` _returnvalue_x))))
      (:`then_1`
        ;[0 0 0] Checking if both players finished level
        (if (`/Game/Blueprints/ThirdPersonCharacter.TouchedFinish` _output)
          (if (`/Game/Blueprints/ThirdPersonCharacter.TouchedFinish` _output_2)
            (set `self.LevelFinished` true)
            (`KismetSystemLibrary.Delay` 0.2)
            (set `/Game/Blueprints/ThirdPersonCharacter.TouchedFinish` false _output)
            (set `/Game/Blueprints/ThirdPersonCharacter.TouchedFinish` false _output_2)
            (set `self.LevelFinished` false)))))))

(event `NoiseDecreaser`
  ;[0 1 0.9753] Function to decrease noise
  (if (> (`self.NoiseCurrentValue`) 0.0)
    (set `self.NoiseCurrentValue` (- (`self.NoiseCurrentValue`) 0.0002))))

(event `PlayersArray`
  ;[0.3 0.3762 1] Put both players in array (for easier referencing)
  (`KismetSystemLibrary.Delay` 0.05)
  (bind _outactors (`GameplayStatics.GetAllActorsOfClass` "/Game/Blueprints/ThirdPersonCharacter.ThirdPersonCharacter_C"))
  (set `self.Characters` _outactors)
  (`KismetSystemLibrary.Delay` 0.02)
  (set `self.CompletedSearch` true))

(event `TimeIncreaser`
  (if (`self.TimerRunning`)
    (set `self.Game_CurrentTime` (+ (`self.Game_CurrentTime`) 0.02))))

(event `AddToNoise`
  (params (AddNoiseValue :type "Float (double-precision)"))
  (set `self.NoiseCurrentValue` (+ AddNoiseValue (`self.NoiseCurrentValue`))))

(event `PoolNoiser`
  (set `self.NoiseCurrentValue` (+ (`self.NoiseCurrentValue`) 0.0006)))

(event `SprinklerNoiser`
  (set `self.NoiseCurrentValue` (+ (`self.NoiseCurrentValue`) 0.0008)))

(event `PoolStart`
  (bind _returnvalue (`KismetSystemLibrary.K2_SetTimer` null "PoolNoiser" 0.01 true)))

(event `PoolStop`
  (`KismetSystemLibrary.K2_ClearAndInvalidateTimerHandle` (stale `PoolStart` _returnvalue)))

(event `SprinklerStart`
  (bind _returnvalue (`KismetSystemLibrary.K2_SetTimer` null "SprinklerNoiser" 0.01 true)))

(event `SprinklerStop`
  (`KismetSystemLibrary.K2_ClearAndInvalidateTimerHandle` (stale `SprinklerStart` _returnvalue)))

(fn `UserConstructionScript`)