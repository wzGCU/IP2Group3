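; SkateboardUp is an obstacle actor that knocks the player and adds noise when hit.
; When a ThirdPersonCharacter enters TriggerVolume, it fires once, launching the character along negative world Y and playing a hit sound.
; It then adds to the noise value in DrunkGameState and destroys itself.
; Separate events show or clear the skateboard on ProperMesh by setting or emptying its static mesh.
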(event `SkateboardUpClearMesh`
  (`StaticMeshComponent.SetStaticMesh` (`self.ProperMesh`) null))

(event `SkateboardUpShow`
  (`StaticMeshComponent.SetStaticMesh` (`self.ProperMesh`) "/Game/Meshes/Placeholders/Skate.Skate"))

(event `self.TriggerVolume.OnComponentBeginOverlap`
  (params (OverlappedComponent :type "PrimitiveComponent Object Reference") (OtherActor :type "Actor Object Reference") (OtherComp :type "PrimitiveComponent Object Reference") (OtherBodyIndex :type Integer) (bFromSweep :type Boolean) (SweepResult :type "HitResult Structure (by ref)"))
  (bind _asthird_person_character (cast `/Game/Blueprints/ThirdPersonCharacter` OtherActor))
  (`/Engine/EditorBlueprintResources/StandardMacros.DoOnce` false
    (:`Completed`
      (`Character.LaunchCharacter` _asthird_person_character (0.0 -1000.0 0.0) false false)
      (`GameplayStatics.PlaySoundAtLocation` "/Game/Audios/ObstacleHit.ObstacleHit" (`SceneComponent.K2_GetComponentLocation` (`self.ProperMesh`)) (struct) 1.0 1.0 0.0 null null null)
      (bind _asdrunk_game_state (cast `/Game/Blueprints/GameMode/DrunkGameState` (`GameplayStatics.GetGameState`)))
      (`/Game/Blueprints/GameMode/DrunkGameState.AddToNoise` _asdrunk_game_state 0.3)
      (`self.K2_DestroyActor`))))

(fn `UserConstructionScript`)