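; Yard door Blueprint that swings open when the player's ThirdPersonCharacter enters its front trigger.
; The overlap starts a looping function timer that steps the door's relative yaw down each tick until it reaches -90 degrees, then clears itself.
; A separate FenceFallNoiser trigger adds noise to the DrunkGameState once, the first time the character overlaps it.
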(event `DoorOpener`
  (bind _door (`self.Door`))
  (bind (_relativerotation_roll _relativerotation_pitch _relativerotation_yaw) (`KismetMathLibrary.BreakRotator` (`SceneComponent.RelativeRotation` _door)))
  (`SceneComponent.K2_SetRelativeRotation` _door (`KismetMathLibrary.MakeRotator` _relativerotation_roll _relativerotation_pitch (- _relativerotation_yaw 0.5)) false false)
  (if (<= _relativerotation_yaw -90.0)
    (`KismetSystemLibrary.K2_ClearAndInvalidateTimerHandle` (stale `self.FrontDoor.OnComponentBeginOverlap` _returnvalue))))

(event `self.FrontDoor.OnComponentBeginOverlap`
  (params (OverlappedComponent :type "PrimitiveComponent Object Reference") (OtherActor :type "Actor Object Reference") (OtherComp :type "PrimitiveComponent Object Reference") (OtherBodyIndex :type Integer) (bFromSweep :type Boolean) (SweepResult :type "HitResult Structure (by ref)"))
  (cast `/Game/Blueprints/ThirdPersonCharacter` OtherActor)
  (bind _returnvalue (`KismetSystemLibrary.K2_SetTimer` null "DoorOpener" 0.001 true)))

(event `self.FenceFallNoiser.OnComponentBeginOverlap`
  (params (OverlappedComponent :type "PrimitiveComponent Object Reference") (OtherActor :type "Actor Object Reference") (OtherComp :type "PrimitiveComponent Object Reference") (OtherBodyIndex :type Integer) (bFromSweep :type Boolean) (SweepResult :type "HitResult Structure (by ref)"))
  (cast `/Game/Blueprints/ThirdPersonCharacter` OtherActor)
  (`/Engine/EditorBlueprintResources/StandardMacros.DoOnce` false
    (:`Completed`
      (bind _asdrunk_game_state (cast `/Game/Blueprints/GameMode/DrunkGameState` (`GameplayStatics.GetGameState`)))
      (`/Game/Blueprints/GameMode/DrunkGameState.AddToNoise` _asdrunk_game_state 0.2))))

(fn `UserConstructionScript`)