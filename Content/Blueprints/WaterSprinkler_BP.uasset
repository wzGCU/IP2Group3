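; Water sprinkler hazard that spins and notifies ThirdPersonCharacter when it enters or leaves either of two box triggers.
; At BeginPlay, authority randomly picks the player visibility tag (P1Vis or P2Vis), spin direction and whether the second arm is destroyed, while remotes briefly delay before applying these values.
; A looping timer rotates the arrow components.
; Separate events show or clear the sprinkler meshes, though clearing skips the third mesh.
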(event `SprinklerClearMesh`
  (`StaticMeshComponent.SetStaticMesh` (`self.sprinkler2`) null)
  (`StaticMeshComponent.SetStaticMesh` (`self.sprinkler1`) null))

(event `SprinklerShow`
  (`StaticMeshComponent.SetStaticMesh` (`self.sprinkler2`) "/Game/Meshes/Final/ObstaclesNCollectibles/C12_Sprinkler_water.C12_Sprinkler_water")
  (`StaticMeshComponent.SetStaticMesh` (`self.sprinkler1`) "/Game/Meshes/Final/ObstaclesNCollectibles/C12_Sprinkler.C12_Sprinkler")
  (`StaticMeshComponent.SetStaticMesh` (`self.sprinkler3`) "/Game/Meshes/Final/ObstaclesNCollectibles/C12_Sprinkler_water.C12_Sprinkler_water"))

(event `WaterRotator`
  (bind _arrow1 (`self.Arrow1`))
  (bind _arrow (`self.Arrow`))
  (bind (_relativerotation_roll _relativerotation_pitch _relativerotation_yaw) (`KismetMathLibrary.BreakRotator` (`SceneComponent.RelativeRotation` _arrow)))
  (bind (_relativerotation_roll_2 _relativerotation_pitch_2 _relativerotation_yaw_2) (`KismetMathLibrary.BreakRotator` (`SceneComponent.RelativeRotation` _arrow1)))
  (`SceneComponent.K2_SetRelativeRotation` _arrow (`KismetMathLibrary.MakeRotator` _relativerotation_roll _relativerotation_pitch (+ _relativerotation_yaw (`self.Speed`))) false false)
  (if (not (> (`self.SprinklersDefiner`) 50.0))
    (`SceneComponent.K2_SetRelativeRotation` _arrow1 (`KismetMathLibrary.MakeRotator` _relativerotation_roll_2 _relativerotation_pitch_2 (+ _relativerotation_yaw_2 (`self.Speed`))) false false)))

(event `self.ReceiveBeginPlay`
  (bind _returnvalue (`KismetMathLibrary.RandomFloatInRange` 0.0 100.0))
  (bind _returnvalue_2 (`ActorComponent.GetOwner` (`self.StaticMeshComponent`)))
  (`KismetSystemLibrary.Delay` 0.2)
  (`/Engine/EditorBlueprintResources/ActorMacros.Switch Has Authority`
    (:`Authority`
      (set `self.RandomAssign` _returnvalue)
      (set `self.RotationDefiner` _returnvalue)
      (set `self.SprinklersDefiner` _returnvalue))
    (:`Remote`
      (`KismetSystemLibrary.Delay` 0.2)))
  (`|ExecutionSequence`
    (:`then_0`
      (if (> (`self.RandomAssign`) 50.0)
        (set `Actor.Tags` (`|MakeArray` "VisibilityBased" "P1Vis" :!type "Name") _returnvalue_2)
        (else
          (set `Actor.Tags` (`|MakeArray` "VisibilityBased" "P2Vis" :!type "Name") _returnvalue_2)))
      (`KismetSystemLibrary.K2_SetTimer` null "WaterRotator" 0.01 true))
    (:`then_1`
      (if (> (`self.RotationDefiner`) 50.0)
        (set `self.Speed` -0.5)
        (else
          (set `self.Speed` 0.5))))
    (:`then_2`
      (if (> (`self.SprinklersDefiner`) 50.0)
        (`ActorComponent.K2_DestroyComponent` (`self.Arrow1`))))))

(event `self.Box.OnComponentBeginOverlap`
  (params (OverlappedComponent :type "PrimitiveComponent Object Reference") (OtherActor :type "Actor Object Reference") (OtherComp :type "PrimitiveComponent Object Reference") (OtherBodyIndex :type Integer) (bFromSweep :type Boolean) (SweepResult :type "HitResult Structure (by ref)"))
  (bind _asthird_person_character (cast `/Game/Blueprints/ThirdPersonCharacter` OtherActor))
  (`/Game/Blueprints/ThirdPersonCharacter.SprinklerEnter` _asthird_person_character))

(event `self.Box.OnComponentEndOverlap`
  (params (OverlappedComponent :type "PrimitiveComponent Object Reference") (OtherActor :type "Actor Object Reference") (OtherComp :type "PrimitiveComponent Object Reference") (OtherBodyIndex :type Integer))
  (bind _asthird_person_character (cast `/Game/Blueprints/ThirdPersonCharacter` OtherActor))
  (`/Game/Blueprints/ThirdPersonCharacter.SprinklerStop` _asthird_person_character))

(event `self.Box1.OnComponentBeginOverlap`
  (params (OverlappedComponent :type "PrimitiveComponent Object Reference") (OtherActor :type "Actor Object Reference") (OtherComp :type "PrimitiveComponent Object Reference") (OtherBodyIndex :type Integer) (bFromSweep :type Boolean) (SweepResult :type "HitResult Structure (by ref)"))
  (bind _asthird_person_character (cast `/Game/Blueprints/ThirdPersonCharacter` OtherActor))
  (`/Game/Blueprints/ThirdPersonCharacter.SprinklerEnter` _asthird_person_character))

(event `self.Box1.OnComponentEndOverlap`
  (params (OverlappedComponent :type "PrimitiveComponent Object Reference") (OtherActor :type "Actor Object Reference") (OtherComp :type "PrimitiveComponent Object Reference") (OtherBodyIndex :type Integer))
  (bind _asthird_person_character (cast `/Game/Blueprints/ThirdPersonCharacter` OtherActor))
  (`/Game/Blueprints/ThirdPersonCharacter.SprinklerStop` _asthird_person_character))

(fn `UserConstructionScript`)