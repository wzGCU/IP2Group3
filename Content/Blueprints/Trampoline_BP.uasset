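; Trampoline actor that launches an overlapping third-person character, plays a sound and adds to the game state's noise.
; Tick watches the launched character and applies a timed stun once it is moving on the ground again.
; On BeginPlay the authority rolls a random value, remotes wait briefly, and the actor gets tagged as visibility-based for P1 or P2.
; Custom events show or clear its mesh and material.
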(event `TrampolineClearMesh`
  (bind _trampoline (`self.Trampoline`))
  (`StaticMeshComponent.SetStaticMesh` _trampoline null)
  (`PrimitiveComponent.SetMaterial` _trampoline 0 null))

(event `TrampolineShow`
  (bind _trampoline (`self.Trampoline`))
  (`StaticMeshComponent.SetStaticMesh` _trampoline "/Game/Meshes/Placeholders/Trampoline.Trampoline")
  (`PrimitiveComponent.SetMaterial` _trampoline 0 "/Game/Materials/TrampolineMat.TrampolineMat"))

(event `self.ReceiveTick`
  (params (DeltaSeconds :type "Float (single-precision)"))
  (if (`self.Launched`)
    (if (`NavMovementComponent.IsMovingOnGround` (`Character.CharacterMovement` (stale `self.Trigger.OnComponentBeginOverlap` _asthird_person_character)))
      (set `self.Launched` false)
      (bind _asthird_person_character (cast `/Game/Blueprints/ThirdPersonCharacter` (stale `self.Trigger.OnComponentBeginOverlap` OtherActor)))
      (`/Game/Blueprints/ThirdPersonCharacter.StunCharacter` _asthird_person_character 3.0))))

(event `self.Trigger.OnComponentBeginOverlap`
  (params (OverlappedComponent :type "PrimitiveComponent Object Reference") (OtherActor :type "Actor Object Reference") (OtherComp :type "PrimitiveComponent Object Reference") (OtherBodyIndex :type Integer) (bFromSweep :type Boolean) (SweepResult :type "HitResult Structure (by ref)"))
  (bind _asthird_person_character (cast `/Game/Blueprints/ThirdPersonCharacter` OtherActor))
  (bind (_returnvalue_x _returnvalue_y) (`KismetMathLibrary.BreakVector` (`self.GetVelocity` _asthird_person_character)))
  (`Character.LaunchCharacter` _asthird_person_character (`KismetMathLibrary.MakeVector` 280.0 (* _returnvalue_y 1.5) 500.0) true true)
  (`GameplayStatics.PlaySoundAtLocation` "/Game/Audios/Trampoline.Trampoline" (`SceneComponent.K2_GetComponentLocation` (`self.Trampoline`)) (struct) 1.0 1.0 0.0 null null null)
  (bind _asdrunk_game_state (cast `/Game/Blueprints/GameMode/DrunkGameState` (`GameplayStatics.GetGameState`)))
  (`/Game/Blueprints/GameMode/DrunkGameState.AddToNoise` _asdrunk_game_state 0.1)
  (set `self.Launched` true))

(event `self.ReceiveBeginPlay`
  (bind _returnvalue (`ActorComponent.GetOwner` (`self.DefaultSceneRoot`)))
  (`KismetSystemLibrary.Delay` 0.2)
  (`/Engine/EditorBlueprintResources/ActorMacros.Switch Has Authority`
    (:`Authority`
      (set `self.RandomAssign` (`KismetMathLibrary.RandomFloatInRange` 0.0 100.0)))
    (:`Remote`
      (`KismetSystemLibrary.Delay` 0.2)))
  (if (> (`self.RandomAssign`) 50.0)
    (set `Actor.Tags` (`|MakeArray` "VisibilityBased" "P1Vis" :!type "Name") _returnvalue)
    (else
      (set `Actor.Tags` (`|MakeArray` "VisibilityBased" "P2Vis" :!type "Name") _returnvalue))))

(fn `UserConstructionScript`)