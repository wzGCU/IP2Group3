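; A water sprinkler hazard that raises the noise level in DrunkGameState while the player overlaps it.
; Looping timers spin its Arrow in a direction chosen randomly at BeginPlay and periodically check the overlap flag, adding noise through a delay-reset DoOnce.
; ThirdPersonCharacter overlaps set that flag and play a Pool sound on entry.
; A separate SprinklerShow event assigns the sprinkler and cone meshes.
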(event `SprinklerShow`
  (`StaticMeshComponent.SetStaticMesh` (`self.sprinkler2`) "/Game/Meshes/Placeholders/Cone.Cone")
  (`StaticMeshComponent.SetStaticMesh` (`self.sprinkler1`) "/Game/Meshes/Placeholders/Sprinkler.Sprinkler"))

(event `WaterRotator`
  (bind _arrow (`self.Arrow`))
  (bind (_relativerotation_roll _relativerotation_pitch _relativerotation_yaw) (`KismetMathLibrary.BreakRotator` (`SceneComponent.RelativeRotation` _arrow)))
  (`SceneComponent.K2_SetRelativeRotation` _arrow (`KismetMathLibrary.MakeRotator` _relativerotation_roll _relativerotation_pitch (+ _relativerotation_yaw (`self.RotationDefiner`))) false false))

(event `self.ReceiveBeginPlay`
  (if (`KismetMathLibrary.RandomBool`)
    (set `self.RotationDefiner` 0.5)
    (else
      (set `self.RotationDefiner` -0.5)))
  (`KismetSystemLibrary.K2_SetTimer` null "WaterRotator" 0.01 true)
  (`KismetSystemLibrary.K2_SetTimer` null "WaterTicker" 0.5 true))

(event `self.ReceiveActorEndOverlap`
  (params (OtherActor :type "Actor Object Reference"))
  (if (== (`GameplayStatics.GetObjectClass` OtherActor) "/Game/Blueprints/ThirdPersonCharacter.ThirdPersonCharacter_C")
    (set `self.PlayerConnects` false)))

(event `self.ReceiveActorBeginOverlap`
  (params (OtherActor :type "Actor Object Reference"))
  (if (== (`GameplayStatics.GetObjectClass` OtherActor) "/Game/Blueprints/ThirdPersonCharacter.ThirdPersonCharacter_C")
    (set `self.PlayerConnects` true)
    (`GameplayStatics.PlaySoundAtLocation` "/Game/Throwaways/Pool.Pool" (`SceneComponent.K2_GetComponentLocation` (`self.sprinkler1`)) (struct) 1.0 1.0 0.0 null null null)))

(event `WaterTicker`
  (if (`self.PlayerConnects`)
    (bind _asdrunk_game_state (cast `/Game/Blueprints/GameMode/DrunkGameState` (`GameplayStatics.GetGameState`)))
    (`/Engine/EditorBlueprintResources/StandardMacros.DoOnce` false :!label _label
      (:`Completed`
        (set `/Game/Blueprints/GameMode/DrunkGameState.NoiseCurrentValue` (+ (`/Game/Blueprints/GameMode/DrunkGameState.NoiseCurrentValue` _asdrunk_game_state) 0.1) _asdrunk_game_state)
        (`KismetSystemLibrary.Delay` 0.5)
        (goto _label :!via `Reset`)))))

(fn `UserConstructionScript`)