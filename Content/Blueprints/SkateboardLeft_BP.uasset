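; A skateboard hazard actor that launches an overlapping third-person character along negative X, plays a hit sound, adds to game-state noise, then destroys itself.
; BeginPlay polls the game state until BothIn, then tags the actor as visibility-based for P1 or P2.
; The authority rolls that assignment randomly, while remotes wait longer before reading the value.
; Custom events show or clear the skateboard mesh.
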(event `SkateboardLeftClearMesh`
  (`StaticMeshComponent.SetStaticMesh` (`self.ProperMesh`) null))

(event `SkateboardLeftShow`
  (`StaticMeshComponent.SetStaticMesh` (`self.ProperMesh`) "/Game/Meshes/ObstaclesNCollectibles/C12_Skateboard.C12_Skateboard"))

(event `self.TriggerVolume.OnComponentBeginOverlap`
  (params (OverlappedComponent :type "PrimitiveComponent Object Reference") (OtherActor :type "Actor Object Reference") (OtherComp :type "PrimitiveComponent Object Reference") (OtherBodyIndex :type Integer) (bFromSweep :type Boolean) (SweepResult :type "HitResult Structure (by ref)"))
  (bind _asthird_person_character (cast `/Game/Blueprints/ThirdPersonCharacter` OtherActor))
  (`/Engine/EditorBlueprintResources/StandardMacros.DoOnce` false
    (:`Completed`
      (`Character.LaunchCharacter` _asthird_person_character (-3000.0 0.0 0.0) false false)
      (`GameplayStatics.PlaySoundAtLocation` "/Game/Audios/Cues/C_Hit.C_Hit" (`SceneComponent.K2_GetComponentLocation` (`self.ProperMesh`)) (struct) 1.0 1.0 0.0 null null null)
      (bind _asdrunk_game_state (cast `/Game/Blueprints/GameMode/DrunkGameState` (`GameplayStatics.GetGameState`)))
      (`/Game/Blueprints/GameMode/DrunkGameState.AddToNoise` _asdrunk_game_state 0.1)
      (`self.K2_DestroyActor`))))

(event `self.ReceiveBeginPlay`
  (bind _returnvalue (`ActorComponent.GetOwner` (`self.DefaultSceneRoot`)))
  (`KismetSystemLibrary.Delay` 1.0 :!label _label)
  (bind _asdrunk_game_state (cast `/Game/Blueprints/GameMode/DrunkGameState` (`GameplayStatics.GetGameState`) :!label _label_2)
    (:`then`
      (if (`/Game/Blueprints/GameMode/DrunkGameState.BothIn` _asdrunk_game_state)
        (`/Engine/EditorBlueprintResources/ActorMacros.Switch Has Authority`
          (:`Authority`
            (set `self.RandomAssign` (`KismetMathLibrary.RandomFloatInRange` 0.0 100.0))
            (`KismetSystemLibrary.Delay` 1.0))
          (:`Remote`
            (`KismetSystemLibrary.Delay` 2.0)))
        (if (> (`self.RandomAssign`) 50.0)
          (set `Actor.Tags` (`|MakeArray` "VisibilityBased" "P1Vis" :!type "Name") _returnvalue)
          (else
            (set `Actor.Tags` (`|MakeArray` "VisibilityBased" "P2Vis" :!type "Name") _returnvalue)))
        (else
          (goto _label))))
    (:`CastFailed`
      (`KismetSystemLibrary.Delay` 2.0)
      (goto _label_2))))

(fn `UserConstructionScript`)