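; DrunkGameState, apparently a game state, tracks how far each of two players has progressed along the world X axis.
; The PlayersArray event waits briefly, gathers all ThirdPersonCharacter actors into an array, then sets a completion flag after a second delay.
; Once that flag is set, Tick copies the X location of the first two characters into the player one and player two progress variables.
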(event `PlayersArray`
  (`KismetSystemLibrary.Delay` 0.2)
  (bind _outactors (`GameplayStatics.GetAllActorsOfClass` "/Game/Blueprints/ThirdPersonCharacter.ThirdPersonCharacter_C"))
  (set `self.Characters` _outactors)
  (`KismetSystemLibrary.Delay` 1.0)
  (set `self.CompletedSearch` true))

(event `self.ReceiveTick`
  (params (DeltaSeconds :type "Float (single-precision)"))
  (bind _returnvalue_x (`KismetMathLibrary.BreakVector` (`SceneComponent.K2_GetComponentLocation` (`Actor.RootComponent` (`|GetArrayItem` (`self.Characters`) 1)))))
  (bind _returnvalue_x_2 (`KismetMathLibrary.BreakVector` (`SceneComponent.K2_GetComponentLocation` (`Actor.RootComponent` (`|GetArrayItem` (`self.Characters`))))))
  (if (`self.CompletedSearch`)
    (`|ExecutionSequence`
      (:`then_0`
        (set `self.PlayerOneProgress` _returnvalue_x_2))
      (:`then_1`
        (set `self.PlayerTwoProgress` _returnvalue_x)))))

(fn `UserConstructionScript`)