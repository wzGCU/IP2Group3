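; Flower collectible actor that increments the game state's collected count when the third-person character overlaps it.
; On first pickup it plays a sound, shrinks on a looping timer for a second, then destroys itself.
; BeginPlay polls the game state until BothIn, then the authority rolls a random value that picks P1 or P2 visibility tags, with remotes delaying before tagging.
; Separate events show or clear the flower mesh.
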(event `FlowerClearMesh`
  (`StaticMeshComponent.SetStaticMesh` (`self.FlowerMesh`) null))

(event `FlowerShow`
  (`StaticMeshComponent.SetStaticMesh` (`self.FlowerMesh`) "/Game/Meshes/ObstaclesNCollectibles/C12_Flower.C12_Flower"))

(event `FlowerSmallizer`
  (bind (_returnvalue_x _returnvalue_y _returnvalue_z) (`KismetMathLibrary.BreakVector` (`self.GetActorScale3D`)))
  (`self.SetActorScale3D` (`KismetMathLibrary.MakeVector` (- _returnvalue_x 0.01) (- _returnvalue_y 0.01) (- _returnvalue_z 0.01))))

(event `self.ReceiveActorBeginOverlap`
  (params (OtherActor :type "Actor Object Reference"))
  (if (== (`GameplayStatics.GetObjectClass` OtherActor) "/Game/Blueprints/ThirdPersonCharacter.ThirdPersonCharacter_C")
    (bind _asdrunk_game_state (cast `/Game/Blueprints/GameMode/DrunkGameState` (`GameplayStatics.GetGameState`)))
    (`/Engine/EditorBlueprintResources/StandardMacros.DoOnce` false
      (:`Completed`
        (set `/Game/Blueprints/GameMode/DrunkGameState.Game_FlowersCollected` (+ (`/Game/Blueprints/GameMode/DrunkGameState.Game_FlowersCollected` _asdrunk_game_state) 1) _asdrunk_game_state)
        (`GameplayStatics.PlaySoundAtLocation` "/Game/Audios/Cues/C_Flower.C_Flower" (`SceneComponent.K2_GetComponentLocation` (`self.FlowerMesh`)) (struct) 1.0 1.0 0.0 null null null)
        (bind _returnvalue (`KismetSystemLibrary.K2_SetTimer` null "FlowerSmallizer" 0.01 true))
        (`KismetSystemLibrary.Delay` 1.0)
        (`KismetSystemLibrary.K2_ClearAndInvalidateTimerHandle` _returnvalue)
        (`self.K2_DestroyActor`)))))

(event `self.ReceiveBeginPlay`
  (bind _returnvalue (`ActorComponent.GetOwner` (`self.StaticMeshComponent`)))
  (`KismetSystemLibrary.Delay` 1.0 :!label _label)
  (bind _asdrunk_game_state (cast `/Game/Blueprints/GameMode/DrunkGameState` (`GameplayStatics.GetGameState`) :!label _label_2)
    (:`then`
      (if (`/Game/Blueprints/GameMode/DrunkGameState.BothIn` _asdrunk_game_state)
        (`/Engine/EditorBlueprintResources/ActorMacros.Switch Has Authority`
          (:`Authority`
            (set `self.RandomAssign` (`KismetMathLibrary.RandomFloatInRange` 0.0 100.0))
            (`KismetSystemLibrary.Delay` 1.0))
          (:`Remote`
            (`KismetSystemLibrary.Delay` 2.0)))
        (if (> (`self.RandomAssign`) 50.0)
          (set `Actor.Tags` (`|MakeArray` "VisibilityBased" "P1Vis" :!type "Name") _returnvalue)
          (else
            (set `Actor.Tags` (`|MakeArray` "VisibilityBased" "P2Vis" :!type "Name") _returnvalue)))
        (else
          (goto _label))))
    (:`CastFailed`
      (`KismetSystemLibrary.Delay` 2.0)
      (goto _label_2))))

(fn `UserConstructionScript`)