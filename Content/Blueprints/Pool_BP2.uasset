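; Pool actor that notifies the ThirdPersonCharacter on entering and leaving its sphere, and takes part in per-player visibility.
; Custom events swap the pool mesh between the visible model and a collision-only version.
; On BeginPlay it polls DrunkGameState until BothIn, then the authority rolls RandomAssign while remotes wait longer.
; The roll tags the actor VisibilityBased plus P1Vis or P2Vis, weighted toward P2.
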(event `PoolClearMesh`
  (`StaticMeshComponent.SetStaticMesh` (`self.ProperPool`) "/Game/Meshes/ObstaclesNCollectibles/C24_PoolCollisionOnly.C24_PoolCollisionOnly"))

(event `PoolShow`
  (`StaticMeshComponent.SetStaticMesh` (`self.ProperPool`) "/Game/Meshes/ObstaclesNCollectibles/C13_Pool.C13_Pool"))

(event `self.Sphere.OnComponentBeginOverlap`
  (params (OverlappedComponent :type "PrimitiveComponent Object Reference") (OtherActor :type "Actor Object Reference") (OtherComp :type "PrimitiveComponent Object Reference") (OtherBodyIndex :type Integer) (bFromSweep :type Boolean) (SweepResult :type "HitResult Structure (by ref)"))
  (bind _asthird_person_character (cast `/Game/Blueprints/ThirdPersonCharacter` OtherActor))
  (`/Game/Blueprints/ThirdPersonCharacter.PoolEnter` _asthird_person_character))

(event `self.Sphere.OnComponentEndOverlap`
  (params (OverlappedComponent :type "PrimitiveComponent Object Reference") (OtherActor :type "Actor Object Reference") (OtherComp :type "PrimitiveComponent Object Reference") (OtherBodyIndex :type Integer))
  (bind _asthird_person_character (cast `/Game/Blueprints/ThirdPersonCharacter` OtherActor))
  (`/Game/Blueprints/ThirdPersonCharacter.PoolStop` _asthird_person_character))

(event `self.ReceiveBeginPlay`
  (bind _returnvalue (`ActorComponent.GetOwner` (`self.StaticMeshComponent`)))
  (`KismetSystemLibrary.Delay` 1.0 :!label _label)
  (bind _asdrunk_game_state (cast `/Game/Blueprints/GameMode/DrunkGameState` (`GameplayStatics.GetGameState`) :!label _label_2)
    (:`then`
      (if (`/Game/Blueprints/GameMode/DrunkGameState.BothIn` _asdrunk_game_state)
        (`/Engine/EditorBlueprintResources/ActorMacros.Switch Has Authority`
          (:`Authority`
            (set `self.RandomAssign` (`KismetMathLibrary.RandomFloatInRange` 0.0 100.0))
            (`KismetSystemLibrary.Delay` 1.0))
          (:`Remote`
            (`KismetSystemLibrary.Delay` 2.0)))
        (if (> (`self.RandomAssign`) 40.0)
          (set `Actor.Tags` (`|MakeArray` "VisibilityBased" "P2Vis" :!type "Name") _returnvalue)
          (else
            (set `Actor.Tags` (`|MakeArray` "VisibilityBased" "P1Vis" :!type "Name") _returnvalue)))
        (else
          (goto _label))))
    (:`CastFailed`
      (`KismetSystemLibrary.Delay` 2.0)
      (goto _label_2))))

(fn `UserConstructionScript`)